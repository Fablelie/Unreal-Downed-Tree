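; Pawn that balances a DownedTrees component between two cubes, like a beam following two end heights.
; The LeftSide axis rewrites the left cube's world Z as a scaled multiple of its current Z; no input here moves the right cube.
; Each tick, DownedTrees takes the cubes' average height and a roll from their clamped height difference, with LeftIsOverRight choosing the tilt direction.
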(event `InputAxis|LeftSide`
  (params (AxisValue :type "Float (single-precision)"))
  (bind (_returnvalue_x _returnvalue_y _returnvalue_z) (`KismetMathLibrary.BreakVector` (`SceneComponent.K2_GetComponentLocation` (`self.CubeLeft`))))
  (`SceneComponent.K2_SetWorldLocation` (`self.CubeLeft`) (`KismetMathLibrary.MakeVector` _returnvalue_x _returnvalue_y (* AxisValue _returnvalue_z 2.0)) false false))

(event `self.ReceiveTick`
  (params (DeltaSeconds :type "Float (single-precision)"))
  (bind _returnvalue (`self.CalculateNewTransform`))
  (`SceneComponent.K2_SetWorldTransform` (`self.DownedTrees`) _returnvalue false false))

(fn `CalculateNewTransform`
  (returns (ReturnValue :type "Transform Structure"))
  (bind (_returnvalue_x _returnvalue_y _returnvalue_z) (`KismetMathLibrary.BreakVector` (`SceneComponent.K2_GetComponentLocation` (`self.CubeLeft`))))
  (bind (_returnvalue_x_2 _returnvalue_y_2 _returnvalue_z_2) (`KismetMathLibrary.BreakVector` (`SceneComponent.K2_GetComponentLocation` (`self.CubeRight`))))
  (bind (_returnvalue_x_3 _returnvalue_y_3 _returnvalue_z_3) (`KismetMathLibrary.BreakVector` (`SceneComponent.K2_GetComponentLocation` (`self.CubeLeft`))))
  (bind (_returnvalue_x_4 _returnvalue_y_4) (`KismetMathLibrary.BreakVector` (`SceneComponent.K2_GetComponentLocation` (`self.DownedTrees`))))
  (bind (_returnvalue_x_5 _returnvalue_y_5 _returnvalue_z_4) (`KismetMathLibrary.BreakVector` (`SceneComponent.K2_GetComponentLocation` (`self.CubeRight`))))
  (return (`KismetMathLibrary.MakeTransform` (`KismetMathLibrary.MakeVector` _returnvalue_x_4 _returnvalue_y_4 (/ (+ _returnvalue_z_4 _returnvalue_z) 2.0)) (`KismetMathLibrary.MakeRotator` (* (`KismetMathLibrary.FClamp` (`KismetMathLibrary.Abs` (- _returnvalue_z_2 _returnvalue_z_3)) 0.0 200.0) 0.05 (`KismetMathLibrary.SelectFloat` 1.0 -1.0 (`self.LeftIsOverRight`)))) (`SceneComponent.K2_GetComponentScale` (`self.DownedTrees`)))))

(fn `UserConstructionScript`)